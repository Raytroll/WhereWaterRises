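; Inventory actor component that adds items to an array of slots, using an item data table for each item's max stack size.
; AddItem visits matching partial stacks first, setting each quantity to the amount moved rather than adding to it.
; Any remainder fills empty "None" slots when IsLimited is set, silently dropping overflow, or otherwise appends new stack-sized slots.
; BeginPlay and Tick are unused.
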(fn `AddItem`
  (params (ItemID :type Name) (Quantity :type Integer))
  (locals (Local_RemainingQuantity :type Integer))
  (bind _returnvalue (> (`local.Local_RemainingQuantity`) 0))
  (bind _returnvalue_2 (`|GetDataTableRow` (`self.Ref_ItemDataTable`) ItemID)
    (:`then`
      (set `local.Local_RemainingQuantity` Quantity)
      (for (_array_element _array_index) (`self.InventoryArray`)
        (bind (_itemid _quantity) (break `/Game/PlayerInventory/Materials/F_InventorySlot` _array_element))
        (bind (_name _type _maxstack) (break `/Game/PlayerInventory/Materials/F_ItemData` _returnvalue_2))
        ; Distributes the quantity of the added item amongst all similar items in the current inventory that have not yet reached their maximum stack size.
        (if (and (== _itemid ItemID) (< _quantity _maxstack))
          (bind _returnvalue_3 (`KismetMathLibrary.Min` (`local.Local_RemainingQuantity`) (- _maxstack _quantity)))
          (`KismetArrayLibrary.Array_Set` (`self.InventoryArray`) _array_index (make `/Game/PlayerInventory/Materials/F_InventorySlot` (`.ItemID_2_F5FA1877424712CE0F12628098B59643` (break `/Game/PlayerInventory/Materials/F_InventorySlot` _array_element)) _returnvalue_3))
          (bind _output_get (set `local.Local_RemainingQuantity` (- (`local.Local_RemainingQuantity`) _returnvalue_3)))
          (if (<= _output_get 0)
            (return))))
      (if _returnvalue
        (if (`self.bIsLimited`)
          ; Fixed Inventory
          (for (_array_element_2 _array_index_2) (`self.InventoryArray`)
            (if (== (`.ItemID_2_F5FA1877424712CE0F12628098B59643` (break `/Game/PlayerInventory/Materials/F_InventorySlot` _array_element_2)) "None")
              (bind _returnvalue_4 (`KismetMathLibrary.Min` (`local.Local_RemainingQuantity`) _maxstack))
              (`KismetArrayLibrary.Array_Set` (`self.InventoryArray`) _array_index_2 (make `/Game/PlayerInventory/Materials/F_InventorySlot` ItemID _returnvalue_4))
              (set `local.Local_RemainingQuantity` (- (`local.Local_RemainingQuantity`) _returnvalue_4))
              (if (== (`local.Local_RemainingQuantity`) 0)
                (return))))
          (return)
          (else
            ; Dynamic Inventory
            (while _returnvalue
              (bind _returnvalue_5 (`KismetMathLibrary.Min` (`local.Local_RemainingQuantity`) _maxstack))
              (`KismetArrayLibrary.Array_Add` (`self.InventoryArray`) (make `/Game/PlayerInventory/Materials/F_InventorySlot` ItemID _returnvalue_5))
              (set `local.Local_RemainingQuantity` (- (`local.Local_RemainingQuantity`) _returnvalue_5)))
            (return)))
        (else
          (return))))
    (:`RowNotFound`
      (return))))