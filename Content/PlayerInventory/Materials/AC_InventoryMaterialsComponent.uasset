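; Inventory component for materials, holding a list of item structs and apparently still unfinished.
; AddItem looks for a matching ItemId, appending a new entry and returning false if that stack is full.
; On overflow it writes the existing element back unchanged, as the remainder and capped-stack calculations are unconnected.
; Merging within the limit, adding unmatched items and CreateInventory have no logic.
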(fn `AddItem`
  (params (Item :type "/Game/PlayerInventory/Materials/F_Item Structure"))
  (returns (IsAdded :type Boolean))
  (bind (_item_id _item_name _item_type _item_currentstack) (break `/Game/PlayerInventory/Materials/F_Item` Item))
  (for (_array_element _array_index) (`self.ListItems`)
    (bind (_item_id_2 _item_name_2 _item_type_2 _item_currentstack_2 _item_maxstack) (break `/Game/PlayerInventory/Materials/F_Item` _array_element))
    (if (== _item_id_2 _item_id)
      (if (== _item_currentstack_2 _item_maxstack)
        (`KismetArrayLibrary.Array_Add` (`self.ListItems`) Item)
        (return false)
        (elif (> (+ _item_currentstack_2 _item_currentstack) _item_maxstack)
          (`KismetArrayLibrary.Array_Set` (`self.ListItems`) _array_index _array_element))))))

(fn `CreateInventory`)