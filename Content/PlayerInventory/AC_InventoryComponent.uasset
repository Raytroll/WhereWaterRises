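; Inventory component that stores items as ID and quantity slots, using either a fixed slot count or a growing array.
; AddItem targets partial stacks, then empty or new slots, capped by the item DataTable's MaxStack.
; RemoveItem walks slots in reverse to reduce or clear them; both functions report results and can fire an inventory-changed dispatcher.
; BeginPlay initializes slots and runs a hardcoded add/remove print test; GetFirstEmptySlot is a stub.
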(event `self.ReceiveBeginPlay`
  (`self.InitializeSlots`)
  ;[0.15 0.000159 0 0.5] AddItem Test
  (bind (_quantityadded _quantityremaining _wasfull) (`self.AddItem` "ID_Sand" 175))
  (`KismetSystemLibrary.PrintString` (`KismetStringLibrary.Concat_StrStr` "Quantity Added : " (`KismetStringLibrary.Conv_IntToString` _quantityadded)))
  (`KismetSystemLibrary.PrintString` (`KismetStringLibrary.Concat_StrStr` "Quantity Remaining : " (`KismetStringLibrary.Conv_IntToString` _quantityremaining)))
  (`KismetSystemLibrary.PrintString` (`KismetStringLibrary.Concat_StrStr` "Was Full : " (`KismetStringLibrary.Conv_BoolToString` _wasfull)))
  (for _array_element (`self.InventoryArray`)
    (bind (_itemid _quantity) (break `/Game/PlayerInventory/F_InventorySlot` _array_element))
    (bind _returnvalue (`|GetDataTableRow` (`self.Ref_ItemDataTable`) _itemid)
      (:`then`
        (`KismetSystemLibrary.PrintString` (`KismetStringLibrary.Concat_StrStr` "Element ADD :" (`KismetTextLibrary.Conv_TextToString` (`.Name_26_03BA56B04C3FA7AD49B6A4AFF069358E` (break `/Game/PlayerInventory/F_ItemData` _returnvalue)))))
        (`KismetSystemLibrary.PrintString` (`KismetStringLibrary.Concat_StrStr` "Element ADD :" (`KismetStringLibrary.Conv_IntToString` _quantity))))))
  (bind (_quantityremoved _quantityremaining_2 _issuccess) (`self.RemoveItem` "ID_Sand" 32))
  (`KismetSystemLibrary.PrintString` (`KismetStringLibrary.Concat_StrStr` "Quantity Removed : " (`KismetStringLibrary.Conv_IntToString` _quantityremoved)))
  (`KismetSystemLibrary.PrintString` (`KismetStringLibrary.Concat_StrStr` "Quantity Remaining (Remove) : " (`KismetStringLibrary.Conv_IntToString` _quantityremaining_2)))
  (`KismetSystemLibrary.PrintString` (`KismetStringLibrary.Concat_StrStr` "Success Removed : " (`KismetStringLibrary.Conv_BoolToString` _issuccess)))
  (for _array_element_2 (`self.InventoryArray`)
    (bind (_itemid_2 _quantity_2) (break `/Game/PlayerInventory/F_InventorySlot` _array_element_2))
    (bind _returnvalue_2 (`|GetDataTableRow` (`self.Ref_ItemDataTable`) _itemid_2)
      (:`then`
        (`KismetSystemLibrary.PrintString` (`KismetStringLibrary.Concat_StrStr` "Element REMOVE :" (`KismetTextLibrary.Conv_TextToString` (`.Name_26_03BA56B04C3FA7AD49B6A4AFF069358E` (break `/Game/PlayerInventory/F_ItemData` _returnvalue_2)))))
        (`KismetSystemLibrary.PrintString` (`KismetStringLibrary.Concat_StrStr` "Element REMOVE :" (`KismetStringLibrary.Conv_IntToString` _quantity_2)))))))

(fn `AddItem`
  (params (ItemID :type Name) (Quantity :type Integer))
  (returns (QuantityAdded :type Integer) (QuantityRemaining :type Integer) (WasFull :type Boolean))
  (locals (Local_RemainingQuantity :type Integer))
  (bind _local_remainingquantity (`local.Local_RemainingQuantity`))
  (bind _returnvalue (> (`local.Local_RemainingQuantity`) 0))
  (bind _returnvalue_2 (`|GetDataTableRow` (`self.Ref_ItemDataTable`) ItemID)
    (:`then`
      (set `local.Local_RemainingQuantity` Quantity)
      (for (_array_element _array_index) (`self.InventoryArray`)
        (bind (_itemid _quantity) (break `/Game/PlayerInventory/F_InventorySlot` _array_element))
        (bind (_name _type _maxstack) (break `/Game/PlayerInventory/F_ItemData` _returnvalue_2))
        ; Distributes the quantity of the added item amongst all similar items in the current inventory that have not yet reached their maximum stack size.
        (if (and (== _itemid ItemID) (< _quantity _maxstack))
          (bind _returnvalue_3 (`KismetMathLibrary.Min` (`local.Local_RemainingQuantity`) (- _maxstack _quantity)))
          (`KismetArrayLibrary.Array_Set` (`self.InventoryArray`) _array_index (make `/Game/PlayerInventory/F_InventorySlot` (`.ItemID_2_F5FA1877424712CE0F12628098B59643` (break `/Game/PlayerInventory/F_InventorySlot` _array_element)) _returnvalue_3))
          (bind _output_get (set `local.Local_RemainingQuantity` (- (`local.Local_RemainingQuantity`) _returnvalue_3)))
          (if (<= _output_get 0)
            (`self.OnInventoryChanged`)
            (return (- Quantity (`local.Local_RemainingQuantity`)) 0 false))))
      (if _returnvalue
        (if (`self.bIsLimited`)
          ; Fixed Inventory
          (for (_array_element_2 _array_index_2) (`self.InventoryArray`)
            (if (== (`.ItemID_2_F5FA1877424712CE0F12628098B59643` (break `/Game/PlayerInventory/F_InventorySlot` _array_element_2)) "None")
              (bind _returnvalue_4 (`KismetMathLibrary.Min` (`local.Local_RemainingQuantity`) _maxstack))
              (`KismetArrayLibrary.Array_Set` (`self.InventoryArray`) _array_index_2 (make `/Game/PlayerInventory/F_InventorySlot` ItemID _returnvalue_4))
              (set `local.Local_RemainingQuantity` (- (`local.Local_RemainingQuantity`) _returnvalue_4))
              (if (== (`local.Local_RemainingQuantity`) 0)
                (`self.OnInventoryChanged`)
                (return (- Quantity (`local.Local_RemainingQuantity`)) 0 false))))
          (return (- Quantity _local_remainingquantity) _local_remainingquantity true)
          (else
            ; Dynamic Inventory
            (while _returnvalue
              (bind _returnvalue_5 (`KismetMathLibrary.Min` (`local.Local_RemainingQuantity`) _maxstack))
              (`KismetArrayLibrary.Array_Add` (`self.InventoryArray`) (make `/Game/PlayerInventory/F_InventorySlot` ItemID _returnvalue_5))
              (set `local.Local_RemainingQuantity` (- (`local.Local_RemainingQuantity`) _returnvalue_5))
              (if (== (`local.Local_RemainingQuantity`) 0)
                (`self.OnInventoryChanged`)
                (return (- Quantity (`local.Local_RemainingQuantity`)) 0 false)))
            (return 0 0 false)))
        (else
          (return 0 0 false))))
    (:`RowNotFound`
      (return 0 Quantity false))))

(fn `GetFirstEmptySlot`
  (returns (FoundIndex :type Boolean))
  (return false))

(fn `InitializeSlots`
  (if (`self.bIsLimited`)
    ; Fixed Inventory
    (for _ (range (`self.MaxSlots`))
      (`KismetArrayLibrary.Array_Add` (`self.InventoryArray`) (make `/Game/PlayerInventory/F_InventorySlot` "None")))
    (else
      ; Dynamic Inventory
      (`KismetArrayLibrary.Array_Clear` (`self.InventoryArray`)))))

(fn `RemoveItem`
  (params (ItemID :type Name) (Quantity :type Integer))
  (returns (QuantityRemoved :type Integer) (QuantityRemaining :type Integer) (IsSuccess :type Boolean))
  (locals (Local_RemainingQuantity :type Integer))
  (bind _returnvalue (`DataTableFunctionLibrary.DoesDataTableRowExist` (`self.Ref_ItemDataTable`) ItemID))
  (if _returnvalue
    (set `local.Local_RemainingQuantity` Quantity)
    (bind (_arrayindex _arrayelement) (`/Engine/EditorBlueprintResources/StandardMacros.ReverseForEachLoop` (`self.InventoryArray`))
      (:`LoopBody`
        (bind (_itemid _quantity) (break `/Game/PlayerInventory/F_InventorySlot` _arrayelement))
        (bind _returnvalue_2 (`KismetMathLibrary.Min` (`local.Local_RemainingQuantity`) _quantity))
        (bind _returnvalue_3 (- _quantity _returnvalue_2))
        (if (and (== _itemid ItemID) (<= _returnvalue_3 0))
          (if (`self.bIsLimited`)
            ; Fixed Inventory
            (`KismetArrayLibrary.Array_Set` (`self.InventoryArray`) _arrayindex (make `/Game/PlayerInventory/F_InventorySlot` "None"))
            (`self.OnInventoryChanged`)
            (return 0 0 true)
            (else
              ; Dynamic Inventory
              (bind _returnvalue_4 (`KismetArrayLibrary.Array_RemoveItem` (`self.InventoryArray`) _arrayelement))
              (`self.OnInventoryChanged`)
              (return 0 0 _returnvalue_4)))
          (else
            ; Distributes the quantity of the removed item amongst all similar items in the current inventory that have not yet reached their maximum stack size.
            (`KismetArrayLibrary.Array_Set` (`self.InventoryArray`) _arrayindex (make `/Game/PlayerInventory/F_InventorySlot` _itemid _returnvalue_3))
            (bind _output_get (set `local.Local_RemainingQuantity` (- (`local.Local_RemainingQuantity`) _returnvalue_2)))
            (if (== _output_get 0)
              (return Quantity 0 true))))))
    (else
      (return 0 Quantity false))))