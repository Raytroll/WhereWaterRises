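; Map manager component that owns building grids and the building actors placed on them, tracked in maps keyed by random digit-string hashes.
; It creates or binds grids, converts world positions into rotated grid cells, and spawns or removes buildings through each grid component.
; Structures can also be placed on the first grid that accepts them.
; Saving writes one slot per grid plus an index save, and loading respawns grids and buildings from it.
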(event `self.ReceiveBeginPlay`)

(fn `BindGrid`
  (params (Target :type "/Game/_WhereWaterRises/Components/AC_GridComponent Object Reference"))
  (returns (OutputPin :type String))
  (bind _hash (`self.GenerateUniqueHash` 16))
  (`BlueprintMapLibrary.Map_Add` (`self.Grids`) _hash Target)
  (`/Game/_WhereWaterRises/Components/AC_GridComponent.BuildGridDataFromInnerActor` Target)
  (return _hash))

(fn `CanPlaceBuildingOnGridAtPosition`
  (params (HashGrid :type String) (Position :type "/Game/_WhereWaterRises/Data/Grid/Struct/F_Vec3I Structure"))
  (returns (success :type Boolean))
  (bind (_value _returnvalue) (`BlueprintMapLibrary.Map_Find` (`self.Grids`) HashGrid))
  (if _returnvalue
    (bind _canplace (`/Game/_WhereWaterRises/Components/AC_GridComponent.CanPlaceBlock` _value Position))
    (return _canplace)
    (else
      (return false))))

(fn `CreateGrid`
  (params (`Grid Metadata` :type "/Game/_WhereWaterRises/Data/Grid/Struct/F_GridMetadata Structure") (PlacableBlocks :type "Set of /Game/_WhereWaterRises/Data/Grid/Struct/F_Vec3I Structure (by ref)"))
  (returns (OutputPin :type String))
  (bind (_position _rotation) (break `/Game/_WhereWaterRises/Data/Grid/Struct/F_GridMetadata` `Grid Metadata`))
  (bind _hash (`self.GenerateUniqueHash` 16))
  (bind _returnvalue (`|SpawnActorFromClass` "/Game/_WhereWaterRises/Blueprints/Grid/BP_Grid.BP_Grid_C" (`KismetMathLibrary.MakeTransform` _position _rotation) "Undefined" "MultiplyWithRoot" null null))
  (bind _returnvalue_2 (`Actor.GetComponentByClass` _returnvalue "/Game/_WhereWaterRises/Components/AC_GridComponent.AC_GridComponent_C"))
  (`BlueprintMapLibrary.Map_Add` (`self.Grids`) _hash _returnvalue_2)
  (`/Game/_WhereWaterRises/Components/AC_GridComponent.SetupPlacableBlocks` _returnvalue_2 PlacableBlocks)
  (return _hash))

(fn `DeserializeGridsFromSave`
  (params (GameSave :type "/Game/_WhereWaterRises/Data/GameSave Object Reference"))
  (`/Game/_WhereWaterRises/Data/GameSave.LoadGrids` GameSave)
  (for (_array_element _array_index) (`/Game/_WhereWaterRises/Data/GameSave.GridsSaveNames` GameSave)
    (`KismetSystemLibrary.PrintString` _array_element true true (struct :`R` 0.050289 :`G` 1.0 :`A` 1.0) 5.0)
    (bind _output (`|GetArrayItem` (`/Game/_WhereWaterRises/Data/GameSave.GridsSave` GameSave) _array_index))
    (bind (_position _rotation) (break `/Game/_WhereWaterRises/Data/Grid/Struct/F_GridMetadata` (`/Game/_WhereWaterRises/Data/GridSave.GridMetadata` _output)))
    (bind _returnvalue (`|SpawnActorFromClass` "/Game/_WhereWaterRises/Blueprints/Grid/BP_Grid.BP_Grid_C" (`KismetMathLibrary.MakeTransform` _position _rotation) "Undefined" "MultiplyWithRoot" null null))
    (bind _ac_buildingcomponent (`/Game/_WhereWaterRises/Blueprints/Grid/BP_Grid.AC_BuildingComponent` _returnvalue))
    (set `/Game/_WhereWaterRises/Components/AC_GridComponent.AvailableBlocks` (`/Game/_WhereWaterRises/Data/GridSave.PlacableBlocks` _output) _ac_buildingcomponent)
    (set `/Game/_WhereWaterRises/Components/AC_GridComponent.GridSize` (`/Game/_WhereWaterRises/Data/GridSave.GridSize` _output) _ac_buildingcomponent)
    (`BlueprintMapLibrary.Map_Add` (`self.Grids`) _array_element _ac_buildingcomponent)
    (set `/Game/_WhereWaterRises/Components/AC_GridComponent.GridData` (`/Game/_WhereWaterRises/Data/GridSave.GridMetadata` _output) _ac_buildingcomponent)
    (bind (_keypin _valuepin) (`|MapForEach` (`/Game/_WhereWaterRises/Data/GridSave.BuildingClasses` _output))
      (:`then`
        (`self.PlaceBuildingFromLocalPosition` _keypin _array_element (`BlueprintMapLibrary.Map_Find` (`/Game/_WhereWaterRises/Data/GridSave.BlocksPositions` _output) _keypin) (`BlueprintMapLibrary.Map_Find` (`/Game/_WhereWaterRises/Data/GridSave.BlocksOrientations` _output) _keypin) _valuepin))))
  (`KismetSystemLibrary.PrintString` "Grids Saves:" true true (struct :`R` 0.050289 :`G` 1.0 :`A` 1.0) 5.0)
  (bind _result (`/Game/_WhereWaterRises/Data/GameSave.GetBuildingCount` GameSave))
  (`KismetSystemLibrary.PrintString` (`KismetStringLibrary.Concat_StrStr` "Buildings: " (`KismetStringLibrary.Conv_IntToString` _result)) true true (struct :`R` 1.0 :`G` 0.140672 :`A` 1.0) 5.0))

(fn `GenerateUniqueHash`
  (params (Size :type Integer))
  (returns (Hash :type String))
  (locals (TempHash :type String))
  (for _ (range (+ Size 1))
    (set `local.TempHash` (`KismetStringLibrary.Concat_StrStr` (`KismetStringLibrary.Conv_IntToString` (`KismetMathLibrary.RandomIntegerInRange` 0 9)) (`local.TempHash`))))
  (return (`local.TempHash`)))

(fn `GetStructurePosition`
  (params (Hash :type String) (GridHash :type String))
  (returns (Position :type "/Game/_WhereWaterRises/Data/Grid/Struct/F_Vec3I Structure") (Success :type Boolean))
  (bind (_value _returnvalue) (`BlueprintMapLibrary.Map_Find` (`self.Grids`) GridHash))
  (if _returnvalue
    (bind (_position _found) (`/Game/_WhereWaterRises/Components/AC_GridComponent.FindBlockPositionByHash` _value Hash))
    (return _position _found)
    (else
      (return (struct) false))))

(fn `LocateStructureOnGrids`
  (params (Hash :type String))
  (returns (GridHash :type String) (Located :type Boolean))
  (bind (_value _returnvalue) (`BlueprintMapLibrary.Map_Find` (`self.BuildingGrid`) Hash))
  (return _value _returnvalue))

(fn `PlaceBuildingFromLocalPosition`
  (params (UniqueHash :type String) (GridHash :type String) (Position :type "/Game/_WhereWaterRises/Data/Grid/Struct/F_Vec3I Structure") (Orientation :type "/Game/_WhereWaterRises/Data/Building/Enumerations/E_BuildingOrientation Enum" :default "NewEnumerator0") (Class :type "Actor Class Reference"))
  (returns (Success :type Boolean))
  (locals (OrientationToRotation :type "Map of /Game/_WhereWaterRises/Data/Building/Enumerations/E_BuildingOrientation Enum to Float (double-precision)"))
  (bind (_x _y _z) (break `/Game/_WhereWaterRises/Data/Grid/Struct/F_Vec3I` Position))
  (bind (_value _returnvalue) (`BlueprintMapLibrary.Map_Find` (`self.Grids`) GridHash))
  (bind (_position _rotation) (break `/Game/_WhereWaterRises/Data/Grid/Struct/F_GridMetadata` (`/Game/_WhereWaterRises/Components/AC_GridComponent.GridData` _value)))
  (if _returnvalue
    (bind _placed (`/Game/_WhereWaterRises/Components/AC_GridComponent.PlaceBlock` _value UniqueHash Position Orientation))
    (if _placed
      (`BlueprintMapLibrary.Map_Add` (`self.BuildingGrid`) UniqueHash GridHash)
      (bind _returnvalue_2 (`|SpawnActorFromClass` Class (`KismetMathLibrary.MakeTransform` (+ _position (`KismetMathLibrary.GreaterGreater_VectorRotator` (* (+ (`KismetMathLibrary.MakeVector` (`KismetMathLibrary.Conv_IntToDouble` _x) (`KismetMathLibrary.Conv_IntToDouble` _y) (`KismetMathLibrary.Conv_IntToDouble` _z)) (0.5 0.5 0.0)) (`/Game/_WhereWaterRises/Components/AC_GridComponent.GridSize` _value)) _rotation)) (`KismetMathLibrary.ComposeRotators` _rotation (`KismetMathLibrary.MakeRotator` 0.0 0.0 (`BlueprintMapLibrary.Map_Find` (`local.OrientationToRotation`) Orientation)))) "Undefined" "MultiplyWithRoot" null null))
      (`BlueprintMapLibrary.Map_Add` (`self.BuildingActor`) UniqueHash _returnvalue_2)
      (`BlueprintSetLibrary.Set_Add` (`self.BuildingHashes`) UniqueHash)
      (return true)
      (else
        (return false)))
    (else
      (return false))))

(fn `PlaceBuildingFromWorldPosition`
  (params (GridHash :type String) (Position :type "Vector Structure") (Orientation :type "/Game/_WhereWaterRises/Data/Building/Enumerations/E_BuildingOrientation Enum" :default "NewEnumerator0") (Class :type "Actor Class Reference"))
  (returns (Hash :type String) (Success :type Boolean))
  (bind (_postitionongrid _worldtransformongrid _success) (`self.ProjectPointOntoGridSpace` Position GridHash))
  (if _success
    (bind _hash (`self.GenerateUniqueHash` 16))
    (bind _success_2 (`self.PlaceBuildingFromLocalPosition` null _hash GridHash _postitionongrid Orientation Class))
    (if _success_2
      (return _hash true)
      (else
        (return "" false)))
    (else
      (return "" false))))

(fn `PlaceStructureAcrossGrids`
  (params (Position :type "Vector Structure") (Orientation :type "/Game/_WhereWaterRises/Data/Building/Enumerations/E_BuildingOrientation Enum" :default "NewEnumerator0") (Class :type "Actor Class Reference"))
  (returns (Hash :type String) (Success :type Boolean))
  (locals (Break :type Boolean))
  (bind _keypin (`|MapForEach` (`self.Grids`))
    (:`then`
      (if (not (`local.Break`))
        (bind (_hash _success) (`self.PlaceBuildingFromWorldPosition` _keypin Position Orientation Class))
        (if _success
          (return _hash true))))
    (:`CompletedPin`
      (return "" false))))

(fn `ProjectPointOntoGridSpace`
  (params (WorldPosition :type "Vector Structure") (GridHash :type String))
  (returns (PostitionOnGrid :type "/Game/_WhereWaterRises/Data/Grid/Struct/F_Vec3I Structure") (WorldTransformOnGrid :type "Transform Structure") (Success :type Boolean))
  (bind (_value _returnvalue) (`BlueprintMapLibrary.Map_Find` (`self.Grids`) GridHash))
  (bind _gridsize (`/Game/_WhereWaterRises/Components/AC_GridComponent.GridSize` _value))
  (bind (_position _rotation) (break `/Game/_WhereWaterRises/Data/Grid/Struct/F_GridMetadata` (`/Game/_WhereWaterRises/Components/AC_GridComponent.GridData` _value)))
  (bind (_returnvalue_x _returnvalue_y _returnvalue_z) (`KismetMathLibrary.BreakVector` (`KismetMathLibrary.TransformLocation` (`KismetMathLibrary.InvertTransform` (`KismetMathLibrary.MakeTransform` _position _rotation)) (`KismetMathLibrary.MakeVector` (.x WorldPosition) (.y WorldPosition) (.z _position)))))
  (bind _returnvalue_2 (`KismetMathLibrary.FFloor` (/ _returnvalue_z _gridsize)))
  (bind _returnvalue_3 (`KismetMathLibrary.FFloor` (/ _returnvalue_x _gridsize)))
  (bind _returnvalue_4 (`KismetMathLibrary.FFloor` (/ _returnvalue_y _gridsize)))
  (if _returnvalue
    (return (make `/Game/_WhereWaterRises/Data/Grid/Struct/F_Vec3I` _returnvalue_3 _returnvalue_4 _returnvalue_2) (`KismetMathLibrary.MakeTransform` (+ _position (`KismetMathLibrary.GreaterGreater_VectorRotator` (* (+ (`KismetMathLibrary.MakeVector` (`KismetMathLibrary.Conv_IntToDouble` _returnvalue_3) (`KismetMathLibrary.Conv_IntToDouble` _returnvalue_4) (`KismetMathLibrary.Conv_IntToDouble` _returnvalue_2)) (0.5 0.5 0.0)) _gridsize) _rotation)) _rotation) true)
    (else
      (return (struct) (struct) false))))

(fn `RemoveBuilding`
  (params (Hash :type String))
  (bind (_value _returnvalue) (`BlueprintMapLibrary.Map_Find` (`self.BuildingGrid`) Hash))
  (bind (_value_2 _returnvalue_2) (`BlueprintMapLibrary.Map_Find` (`self.BuildingActor`) Hash))
  (bind (_value_3 _returnvalue_3) (`BlueprintMapLibrary.Map_Find` (`self.Grids`) _value))
  (if _returnvalue
    (if _returnvalue_3
      (`/Game/_WhereWaterRises/Components/AC_GridComponent.RemoveBlock` _value_3 Hash)
      (`BlueprintSetLibrary.Set_Remove` (`self.BuildingHashes`) Hash)
      (if _returnvalue_2
        (`Actor.K2_DestroyActor` _value_2))
      (`BlueprintMapLibrary.Map_Remove` (`self.BuildingActor`) Hash)
      (`BlueprintMapLibrary.Map_Remove` (`self.BuildingGrid`) Hash))))

(fn `SerializeGrids`
  (params (SaveName :type String))
  (returns (Success :type Boolean))
  (locals (`Building Classes` :type "Map of String to Actor Class Reference") (GridsSaves :type "Array of /Game/_WhereWaterRises/Data/GridSave Object Reference") (GridsSaveNames :type "Array of String"))
  (bind _building_classes (`local.Building Classes`))
  (bind (_keypin _valuepin) (`|MapForEach` (`self.Grids`))
    (:`then`
      (bind _returnvalue (`GameplayStatics.CreateSaveGameObject` "/Game/_WhereWaterRises/Data/GridSave.GridSave_C"))
      (bind _blockspositions (`/Game/_WhereWaterRises/Components/AC_GridComponent.BlocksPositions` _valuepin))
      (set `/Game/_WhereWaterRises/Data/GridSave.BlocksPositions` _blockspositions _returnvalue)
      (set `/Game/_WhereWaterRises/Data/GridSave.BlocksOrientations` (`/Game/_WhereWaterRises/Components/AC_GridComponent.BlocksOrientations` _valuepin) _returnvalue)
      (set `/Game/_WhereWaterRises/Data/GridSave.PlacableBlocks` (`/Game/_WhereWaterRises/Components/AC_GridComponent.PlacableBlocks` _valuepin) _returnvalue)
      (set `/Game/_WhereWaterRises/Data/GridSave.GridSize` (`/Game/_WhereWaterRises/Components/AC_GridComponent.GridSize` _valuepin) _returnvalue)
      (bind _keypin_2 (`|MapForEach` _blockspositions)
        (:`then`
          (if (not (`.ReturnValue` (`BlueprintMapLibrary.Map_Find` _building_classes _keypin_2)))
            (`BlueprintMapLibrary.Map_Add` _building_classes _keypin_2 (`GameplayStatics.GetObjectClass` (`BlueprintMapLibrary.Map_Find` (`self.BuildingActor`) _keypin_2)))))
        (:`CompletedPin`
          (set `/Game/_WhereWaterRises/Data/GridSave.BuildingClasses` (`local.Building Classes`) _returnvalue)
          (set `/Game/_WhereWaterRises/Data/GridSave.GridMetadata` (`/Game/_WhereWaterRises/Components/AC_GridComponent.GridData` (`BlueprintMapLibrary.Map_Find` (`self.Grids`) _keypin)) _returnvalue)
          (`/Game/_WhereWaterRises/Data/GridSave.DebugGridData` _returnvalue)
          (`GameplayStatics.SaveGameToSlot` _returnvalue _keypin)
          (`KismetArrayLibrary.Array_Add` (`local.GridsSaveNames`) _keypin)
          (`BlueprintMapLibrary.Map_Clear` (`local.Building Classes`)))))
    (:`CompletedPin`
      (bind _returnvalue_2 (`GameplayStatics.CreateSaveGameObject` "/Game/_WhereWaterRises/Data/GameSave.GameSave_C"))
      (set `/Game/_WhereWaterRises/Data/GameSave.GridsSaveNames` (`local.GridsSaveNames`) _returnvalue_2)
      (bind _returnvalue_3 (`GameplayStatics.SaveGameToSlot` _returnvalue_2 SaveName))
      (return _returnvalue_3))))