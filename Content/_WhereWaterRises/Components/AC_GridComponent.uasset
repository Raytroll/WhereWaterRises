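; Grid component that tracks placeable cells and placed blocks on its owner actor, including water that can spread.
; It derives integer cells from the owner's static mesh locations divided by grid size.
; Placing and removing blocks updates the free-cell set and hash-keyed position, orientation and class maps, plus a reverse position lookup.
; Water propagation uses a neighbor kernel to skip fully surrounded water and returns free cells beside the rest, without placing blocks.
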(fn `BuildGridDataFromInnerActor`
  (bind _returnvalue (`self.GetOwner`))
  (bind _gridsize (`self.GridSize`))
  (bind _returnvalue_2 (`Actor.K2_GetComponentsByClass` _returnvalue "/Script/Engine.StaticMeshComponent"))
  (`KismetSystemLibrary.PrintString` (`KismetStringLibrary.Concat_StrStr` "Found: " (`KismetStringLibrary.Conv_IntToString` (`KismetArrayLibrary.Array_Length` _returnvalue_2))))
  (for _array_element _returnvalue_2
    (bind (_relativelocation_x _relativelocation_y _relativelocation_z) (`KismetMathLibrary.BreakVector` (`SceneComponent.RelativeLocation` _array_element)))
    (bind _f_vec3i (make `/Game/_WhereWaterRises/Data/Grid/Struct/F_Vec3I` (/ (`KismetMathLibrary.FTrunc` _relativelocation_x) _gridsize) (/ (`KismetMathLibrary.FTrunc` _relativelocation_y) _gridsize) (/ (`KismetMathLibrary.FTrunc` _relativelocation_z) _gridsize)))
    (`BlueprintSetLibrary.Set_Add` (`self.PlacableBlocks`) _f_vec3i)
    (`BlueprintSetLibrary.Set_Add` (`self.AvailableBlocks`) _f_vec3i)
    (`SceneComponent.SetVisibility` _array_element true false))
  (set `self.GridData` (make `/Game/_WhereWaterRises/Data/Grid/Struct/F_GridMetadata` (`Actor.K2_GetActorLocation` _returnvalue) (`Actor.K2_GetActorRotation` _returnvalue))))

(fn `CanPlaceBlock`
  (params (Position :type "/Game/_WhereWaterRises/Data/Grid/Struct/F_Vec3I Structure"))
  (returns (CanPlace :type Boolean))
  (bind (_x _y _z) (break `/Game/_WhereWaterRises/Data/Grid/Struct/F_Vec3I` Position))
  (bind _valuepin (`|SetForEach` (`self.AvailableBlocks`))
    (:`then`
      (bind (_x_2 _y_2 _z_2) (break `/Game/_WhereWaterRises/Data/Grid/Struct/F_Vec3I` _valuepin))
      (if (and (== _x_2 _x) (== _y_2 _y) (== _z_2 _z))
        (return true)))
    (:`CompletedPin`
      (return false))))

(fn `FindBlockPositionByHash`
  (params (Hash :type "String (by ref)"))
  (returns (Position :type "/Game/_WhereWaterRises/Data/Grid/Struct/F_Vec3I Structure") (Found :type Boolean))
  (bind (_value _returnvalue) (`BlueprintMapLibrary.Map_Find` (`self.BlocksPositions`) Hash))
  (return _value _returnvalue))

(fn `InitBuilding`
  (params (Building :type "/Game/_WhereWaterRises/Data/Building/Structs/F_Building Structure (by ref)"))
  (bind _hash (`/Game/_WhereWaterRises/Components/AC_MapManager.GenerateUniqueHash` (`self.MapManager`) 16)))

(fn `PlaceBlock`
  (params (Hash :type String) (Position :type "/Game/_WhereWaterRises/Data/Grid/Struct/F_Vec3I Structure") (Orientation :type "/Game/_WhereWaterRises/Data/Building/Enumerations/E_BuildingOrientation Enum" :default "NewEnumerator0") (Class :type "Actor Class Reference"))
  (returns (Placed :type Boolean))
  (bind _canplace (`self.CanPlaceBlock` Position))
  (if _canplace
    (`BlueprintMapLibrary.Map_Add` (`self.BlocksPositions`) Hash Position)
    (`BlueprintMapLibrary.Map_Add` (`self.BlocksOrientations`) Hash Orientation)
    (`BlueprintMapLibrary.Map_Add` (`self.BlocksClasses`) Hash)
    (`BlueprintMapLibrary.Map_Add` (`self.PositionsBlock`) Position Hash)
    (`BlueprintSetLibrary.Set_Remove` (`self.AvailableBlocks`) Position)
    (if (== Class "/Game/_WhereWaterRises/Blueprints/Building/BP_Water.BP_Water_C")
      (`BlueprintMapLibrary.Map_Add` (`self.BlocksWaterIsEdge`) Hash))
    (return true)
    (else
      (return false))))

(fn `PropagateWater`
  (returns (PropagatedPositions :type "Set of /Game/_WhereWaterRises/Data/Grid/Struct/F_Vec3I Structure"))
  (locals (NewWaterBlockEdgeValues :type "Map of String to Boolean") (NeigbourgKernelCheck :type "Array of /Game/_WhereWaterRises/Data/Grid/Struct/F_Vec3I Structure") (NeibourgsCount :type Integer) (PropagatedPositions :type "Set of /Game/_WhereWaterRises/Data/Grid/Struct/F_Vec3I Structure"))
  (`BlueprintMapLibrary.Map_Clear` (`local.NewWaterBlockEdgeValues`))
  (bind _keypin (`|MapForEach` (`self.BlocksWaterIsEdge`))
    (:`then`
      (set `local.NeibourgsCount` 0)
      (for _array_element (`local.NeigbourgKernelCheck`)
        (bind (_x _y _z) (break `/Game/_WhereWaterRises/Data/Grid/Struct/F_Vec3I` _array_element))
        (bind (_x_2 _y_2 _z_2) (break `/Game/_WhereWaterRises/Data/Grid/Struct/F_Vec3I` (`BlueprintMapLibrary.Map_Find` (`self.BlocksPositions`) _keypin)))
        (if (`.ReturnValue` (`BlueprintMapLibrary.Map_Find` (`self.PositionsBlock`) (make `/Game/_WhereWaterRises/Data/Grid/Struct/F_Vec3I` (+ _x _x_2) (+ _y _y_2) (+ _z _z_2))))
          (`/Engine/EditorBlueprintResources/StandardMacros.IncrementInt` (`local.NeibourgsCount`))))
      (`BlueprintMapLibrary.Map_Add` (`self.BlocksWaterIsEdge`) _keypin (== (`local.NeibourgsCount`) (`KismetArrayLibrary.Array_Length` (`local.NeigbourgKernelCheck`)))))
    (:`CompletedPin`
      (`BlueprintSetLibrary.Set_Clear` (`local.PropagatedPositions`))
      (bind (_keypin_2 _valuepin) (`|MapForEach` (`self.PositionsBlock`))
        (:`then`
          (bind (_value _returnvalue) (`BlueprintMapLibrary.Map_Find` (`self.BlocksWaterIsEdge`) _valuepin))
          (if (and (not _value) _returnvalue)
            (for _array_element_2 (`local.NeigbourgKernelCheck`)
              (bind (_x_3 _y_3 _z_3) (break `/Game/_WhereWaterRises/Data/Grid/Struct/F_Vec3I` _array_element_2))
              (bind (_x_4 _y_4 _z_4) (break `/Game/_WhereWaterRises/Data/Grid/Struct/F_Vec3I` _keypin_2))
              (bind _f_vec3i (make `/Game/_WhereWaterRises/Data/Grid/Struct/F_Vec3I` (+ _x_3 _x_4) (+ _y_3 _y_4) (+ _z_3 _z_4)))
              (if (`BlueprintSetLibrary.Set_Contains` (`self.AvailableBlocks`) _f_vec3i)
                (`BlueprintSetLibrary.Set_Add` (`local.PropagatedPositions`) _f_vec3i)))))
        (:`CompletedPin`
          (return (`local.PropagatedPositions`)))))))

(fn `RemoveBlock`
  (params (Hash :type String))
  (bind _blockspositions (`self.BlocksPositions`))
  (bind (_value _returnvalue) (`BlueprintMapLibrary.Map_Find` _blockspositions Hash))
  (if _returnvalue
    (`BlueprintSetLibrary.Set_Add` (`self.AvailableBlocks`) _value))
  (`BlueprintMapLibrary.Map_Remove` _blockspositions Hash)
  (`BlueprintMapLibrary.Map_Remove` (`self.BlocksOrientations`) Hash)
  (`BlueprintMapLibrary.Map_Remove` (`self.BlocksClasses`) Hash)
  (`BlueprintMapLibrary.Map_Remove` (`self.PositionsBlock`) _value)
  (`BlueprintMapLibrary.Map_Remove` (`self.BlocksWaterIsEdge`) Hash))

(fn `SetupPlacableBlocks`
  (params (PlacableBlocks :type "Set of /Game/_WhereWaterRises/Data/Grid/Struct/F_Vec3I Structure"))
  (bind _valuepin (`|SetForEach` PlacableBlocks)
    (:`then`
      (`BlueprintSetLibrary.Set_Add` (`self.PlacableBlocks`) _valuepin)
      (`BlueprintSetLibrary.Set_Add` (`self.AvailableBlocks`) _valuepin))))