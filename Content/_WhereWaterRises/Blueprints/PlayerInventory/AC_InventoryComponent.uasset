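; Inventory component that stores stacked items in either a fixed-slot or growable array, chosen by IsLimited.
; Adds fill matching stacks before empty or new slots, and removals work from the end, with stack limits and ID validation from an item DataTable.
; A per-item totals cache serves quantity lookups, and change dispatchers announce updates.
; A separate hotbar map binds slot indices to item IDs, moving an item already assigned elsewhere.
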(event `self.ReceiveBeginPlay`
  (`self.InitializeSlots`))

(fn `AddItem`
  (params (ItemID :type Name) (Quantity :type Integer))
  (returns (QuantityAdded :type Integer) (QuantityRemaining :type Integer) (IsInventoryFull :type Boolean))
  (locals (Local_TempQuantityRemaining :type Integer) (Local_RemainingQuantity :type Integer) (Local_SlotsIsVoid :type "Array of Integer") (Local_LastSlotLoop :type Integer) (Local_IsInventoryFull :type Boolean))
  (bind _local_remainingquantity (`local.Local_RemainingQuantity`))
  (bind _local_remainingquantity_2 (`local.Local_RemainingQuantity`))
  (bind _local_remainingquantity_3 (`local.Local_RemainingQuantity`))
  (bind _returnvalue (- Quantity _local_remainingquantity))
  (bind _returnvalue_2 (> (`local.Local_RemainingQuantity`) 0))
  (bind (_itemid _quantity) (break `/Game/_WhereWaterRises/Blueprints/PlayerInventory/Data/F_InventorySlot` (`|GetArrayItem` (`self.InventoryArray`) (`KismetArrayLibrary.Array_LastIndex` (`local.Local_SlotsIsVoid`)))))
  (bind _returnvalue_3 (`|GetDataTableRow` (`self.Ref_ItemDataTable`) ItemID)
    (:`then`
      (set `local.Local_RemainingQuantity` Quantity)
      (for (_array_element _array_index) (`self.InventoryArray`)
        (bind (_name _type _maxstack) (break `/Game/_WhereWaterRises/Blueprints/PlayerInventory/Data/F_ItemData` _returnvalue_3))
        (bind (_itemid_2 _quantity_2) (break `/Game/_WhereWaterRises/Blueprints/PlayerInventory/Data/F_InventorySlot` _array_element))
        (bind _returnvalue_4 (`KismetMathLibrary.Min` (`local.Local_RemainingQuantity`) (- _maxstack _quantity_2)))
        ; Distributes the quantity of the added item amongst all similar items in the current inventory that have not yet reached their maximum stack size.
        (set `local.Local_TempQuantityRemaining` _returnvalue_4)
        (if (and (== _itemid_2 ItemID) (< _quantity_2 _maxstack))
          (`KismetArrayLibrary.Array_Set` (`self.InventoryArray`) _array_index (make `/Game/_WhereWaterRises/Blueprints/PlayerInventory/Data/F_InventorySlot` _itemid_2 (+ _quantity_2 _returnvalue_4)))
          ;; Update ItemTotalsCache
          (bind _isupdate (`self.UpdateItemCache` _itemid_2 (`local.Local_TempQuantityRemaining`)))
          (if _isupdate
            (bind _output_get (set `local.Local_RemainingQuantity` (- (`local.Local_RemainingQuantity`) (`local.Local_TempQuantityRemaining`))))
            (if (<= _output_get 0)
              (break)))
          (elif (== _itemid_2 "None")
            (`KismetArrayLibrary.Array_AddUnique` (`local.Local_SlotsIsVoid`) _array_index))))
      (if _returnvalue_2
        (if (`self.bIsLimited`)
          ;[0.7454 0.6584 0 0.502] Fixed Inventory
          (for _array_element_2 (`local.Local_SlotsIsVoid`)
            (bind _returnvalue_5 (`KismetMathLibrary.Min` (`local.Local_RemainingQuantity`) _maxstack))
            (`KismetArrayLibrary.Array_Set` (`self.InventoryArray`) _array_element_2 (make `/Game/_WhereWaterRises/Blueprints/PlayerInventory/Data/F_InventorySlot` ItemID _returnvalue_5))
            ;; Update ItemTotalsCache
            (bind _isupdate_2 (`self.UpdateItemCache` ItemID _returnvalue_5))
            (if _isupdate_2
              (set `local.Local_RemainingQuantity` (- (`local.Local_RemainingQuantity`) _returnvalue_5))
              (if (== (`local.Local_RemainingQuantity`) 0)
                (`self.OnInventoryChanged`)
                (return _returnvalue (`local.Local_RemainingQuantity`) (`local.Local_IsInventoryFull`)))))
          (if (== (`KismetArrayLibrary.Array_Length` (`local.Local_SlotsIsVoid`)) 0)
            (set `local.Local_IsInventoryFull` true)
            (elif (and (== ItemID _itemid) (< _quantity _maxstack))
              _
              (else
                (bind _output_get_2 (set `local.Local_IsInventoryFull` true))
                (`self.OnInventoryChanged`)
                (return _returnvalue _local_remainingquantity _output_get_2))))
          (`self.OnInventoryChanged`)
          (return _returnvalue _local_remainingquantity (`local.Local_IsInventoryFull`))
          (else
            ;[0.06684 0.6146 0 0.5] Dynamic Inventory
            (while _returnvalue_2
              (bind _returnvalue_6 (`KismetMathLibrary.Min` (`local.Local_RemainingQuantity`) _maxstack))
              (`KismetArrayLibrary.Array_Add` (`self.InventoryArray`) (make `/Game/_WhereWaterRises/Blueprints/PlayerInventory/Data/F_InventorySlot` ItemID _returnvalue_6))
              (bind _isupdate_3 (`self.UpdateItemCache` ItemID _returnvalue_6))
              (if _isupdate_3
                (set `local.Local_RemainingQuantity` (- (`local.Local_RemainingQuantity`) _returnvalue_6))))
            (`self.OnInventoryChanged`)
            (return (- Quantity _local_remainingquantity_3) _local_remainingquantity_3 (`local.Local_IsInventoryFull`))))
        (else
          ; Return if there are no more quantities left to add
          (`self.OnInventoryChanged`)
          (return (- Quantity _local_remainingquantity_2) _local_remainingquantity_2 (`local.Local_IsInventoryFull`)))))
    (:`RowNotFound`
      (return 0 Quantity (`local.Local_IsInventoryFull`)))))

(fn `CanAddItem`
  (params (ItemID :type Name) (Quantity :type Integer))
  (returns (QuantityAccepted :type Integer) (AllQuantityAccepted :type Boolean))
  (locals (Local_TotalSpaceAvailable :type Integer))
  (bind _local_totalspaceavailable (`local.Local_TotalSpaceAvailable`))
  (bind _returnvalue (`|GetDataTableRow` (`self.Ref_ItemDataTable`) ItemID)
    (:`then`
      (if (`self.bIsLimited`)
        (for _array_element (`self.InventoryArray`)
          (bind (_itemid _quantity) (break `/Game/_WhereWaterRises/Blueprints/PlayerInventory/Data/F_InventorySlot` _array_element))
          (bind (_name _type _maxstack) (break `/Game/_WhereWaterRises/Blueprints/PlayerInventory/Data/F_ItemData` _returnvalue))
          (if (and (or (== _itemid ItemID) (== _itemid "None")) (< _quantity _maxstack))
            (set `local.Local_TotalSpaceAvailable` (+ (`local.Local_TotalSpaceAvailable`) (- _maxstack _quantity)))))
        (return (`KismetMathLibrary.Min` _local_totalspaceavailable Quantity) (== _local_totalspaceavailable Quantity))
        (else
          (return Quantity false))))
    (:`RowNotFound`
      (return 0 false))))

(fn `CanRemoveItem`
  (params (ItemID :type Name) (Quantity :type Integer))
  (returns (QuantityAvailable :type Integer) (AllQuantityAccepted :type Boolean))
  (locals (Local_TotalQuantityAvailable :type Integer))
  (bind _local_totalquantityavailable (`local.Local_TotalQuantityAvailable`))
  (bind _returnvalue (`DataTableFunctionLibrary.DoesDataTableRowExist` (`self.Ref_ItemDataTable`) ItemID))
  (if _returnvalue
    (for _array_element (`self.InventoryArray`)
      (bind (_itemid _quantity) (break `/Game/_WhereWaterRises/Blueprints/PlayerInventory/Data/F_InventorySlot` _array_element))
      (if (== _itemid ItemID)
        (set `local.Local_TotalQuantityAvailable` (+ _quantity (`local.Local_TotalQuantityAvailable`)))))
    (return (`KismetMathLibrary.Min` _local_totalquantityavailable Quantity) (== _local_totalquantityavailable Quantity))
    (else
      (return 0 false))))

(fn `GetDataTable`
  (returns (DataTable :type "DataTable Object Reference"))
  (locals (Local_Ref_DataTable :type "DataTable Object Reference"))
  (bind _output_get (set `local.Local_Ref_DataTable` (`self.Ref_ItemDataTable`)))
  (return _output_get))

(fn `GetHotbarSlots`
  (params (SlotIndex :type Integer))
  (returns (ItemID :type Name))
  (bind (_value _returnvalue) (`BlueprintMapLibrary.Map_Find` (`self.HotbarSlots`) SlotIndex))
  (if _returnvalue
    (return _value)
    (else
      (return "None"))))

(fn `GetInventoryArray`
  (returns (InventoryArray :type "Array of /Game/_WhereWaterRises/Blueprints/PlayerInventory/Data/F_InventorySlot Structure"))
  (locals (Local_Ref_InventoryArray :type "Array of /Game/_WhereWaterRises/Blueprints/PlayerInventory/Data/F_InventorySlot Structure"))
  (bind _output_get (set `local.Local_Ref_InventoryArray` (`self.InventoryArray`)))
  (return _output_get))

(fn `GetTotalQuantityByItemID`
  (params (ItemID :type Name))
  (returns (Total :type Integer))
  (bind (_value _returnvalue) (`BlueprintMapLibrary.Map_Find` (`self.ItemTotalsCache`) ItemID))
  (if _returnvalue
    (return _value)
    (else
      (return 0))))

(fn `InitializeSlots`
  (if (`self.bIsLimited`)
    ;[0.7454 0.6584 0 0.502] Fixed Inventory
    (for _ (range (`self.MaxSlots`))
      (`KismetArrayLibrary.Array_Add` (`self.InventoryArray`) (make `/Game/_WhereWaterRises/Blueprints/PlayerInventory/Data/F_InventorySlot` "None")))
    (else
      ;[0.06684 0.6146 0 0.5] Dynamic Inventory
      (`KismetArrayLibrary.Array_Clear` (`self.InventoryArray`)))))

(fn `RemoveItem`
  (params (ItemID :type Name) (Quantity :type Integer))
  (returns (QuantityRemoved :type Integer) (QuantityRemaining :type Integer) (IsSuccess :type Boolean))
  (locals (Local_RemainingQuantity :type Integer) (Local_TempQuantityRemaining :type Integer))
  (bind _local_remainingquantity (`local.Local_RemainingQuantity`))
  (bind _returnvalue (- 0 (`local.Local_TempQuantityRemaining`)))
  (bind _returnvalue_2 (- (`local.Local_RemainingQuantity`) (`local.Local_TempQuantityRemaining`)))
  (bind _returnvalue_3 (`DataTableFunctionLibrary.DoesDataTableRowExist` (`self.Ref_ItemDataTable`) ItemID))
  (if _returnvalue_3
    (set `local.Local_RemainingQuantity` Quantity)
    (bind (_arrayindex _arrayelement) (`/Engine/EditorBlueprintResources/StandardMacros.ReverseForEachLoop` (`self.InventoryArray`))
      (:`LoopBody`
        (bind (_itemid _quantity) (break `/Game/_WhereWaterRises/Blueprints/PlayerInventory/Data/F_InventorySlot` _arrayelement))
        ; Verifiy that the item matches the slot and that there is sufficient space remaining
        (if (== _itemid ItemID)
          (bind _returnvalue_4 (`KismetMathLibrary.Min` (`local.Local_RemainingQuantity`) _quantity))
          (set `local.Local_TempQuantityRemaining` _returnvalue_4)
          (bind _returnvalue_5 (- _quantity _returnvalue_4))
          (if (> _returnvalue_5 0)
            ; Distributes the quantity of the removed item amongst all similar items in the current inventory that have not yet reached their maximum stack size.
            (`KismetArrayLibrary.Array_Set` (`self.InventoryArray`) _arrayindex (make `/Game/_WhereWaterRises/Blueprints/PlayerInventory/Data/F_InventorySlot` _itemid _returnvalue_5))
            ;; Update ItemTotalsCache
            (bind _isupdate (`self.UpdateItemCache` _itemid _returnvalue))
            (if _isupdate
              (bind _output_get (set `local.Local_RemainingQuantity` (- (`local.Local_RemainingQuantity`) (`local.Local_TempQuantityRemaining`))))
              (if (<= _output_get 0)
                (`self.OnInventoryChanged`)
                (return Quantity _output_get true)))
            (elif (`self.bIsLimited`)
              ;[0.7454 0.6584 0 0.502] Fixed Inventory
              (`KismetArrayLibrary.Array_Set` (`self.InventoryArray`) _arrayindex (make `/Game/_WhereWaterRises/Blueprints/PlayerInventory/Data/F_InventorySlot` "None"))
              ;; Update ItemTotalsCache
              (bind _isupdate_2 (`self.UpdateItemCache` ItemID _returnvalue))
              (if _isupdate_2
                (bind _output_get_2 (set `local.Local_RemainingQuantity` _returnvalue_2))
                (if (== _output_get_2 0)
                  (`self.OnInventoryChanged`)
                  (return 0 0 true)))
              (else
                ;[0.06684 0.6146 0 0.5] Dynamic Inventory
                (`KismetArrayLibrary.Array_Remove` (`self.InventoryArray`) _arrayindex)
                ;; Update ItemTotalsCache
                (`self.UpdateItemCache` ItemID _returnvalue)
                (if true
                  (bind _output_get_3 (set `local.Local_RemainingQuantity` _returnvalue_2))
                  (if (== _output_get_3 0)
                    (`self.OnInventoryChanged`)
                    (return 0 0 true))))))))
      (:`Completed`
        (`self.OnInventoryChanged`)
        (return (- Quantity _local_remainingquantity) _local_remainingquantity true)))
    (else
      (return 0 Quantity false))))

(fn `SetHotbarItem`
  (params (SlotIndex :type Integer) (DraggedItemID :type Name) (DraggedItemIcon :type "Texture2D Object Reference"))
  (locals (Local_OldSlotIndex :type Integer :default -1))
  (bind _local_oldslotindex (`local.Local_OldSlotIndex`))
  (bind (_keypin _valuepin) (`|MapForEach` (`self.HotbarSlots`) :!label _label)
    (:`then`
      (if (== _valuepin DraggedItemID)
        (set `local.Local_OldSlotIndex` _keypin)
        (goto _label :!via `BreakPin`)))
    (:`CompletedPin`
      (if (> (`local.Local_OldSlotIndex`) -1)
        (`BlueprintMapLibrary.Map_Remove` (`self.HotbarSlots`) _local_oldslotindex)
        (`self.OnHotbarChanged` _local_oldslotindex))
      (`BlueprintMapLibrary.Map_Add` (`self.HotbarSlots`) SlotIndex DraggedItemID)
      (`self.OnHotbarChanged` SlotIndex DraggedItemID DraggedItemIcon)
      (return))))

(fn `UpdateItemCache`
  (params (ItemID :type Name) (Amount :type Integer))
  (returns (IsUpdate :type Boolean))
  (bind _itemtotalscache (`self.ItemTotalsCache`))
  (bind (_value _returnvalue) (`BlueprintMapLibrary.Map_Find` (`self.ItemTotalsCache`) ItemID))
  (bind _returnvalue_2 (+ Amount _value))
  (if _returnvalue
    (if (<= _returnvalue_2 0)
      (bind _returnvalue_3 (`BlueprintMapLibrary.Map_Remove` _itemtotalscache ItemID))
      (return _returnvalue_3)
      (else
        (`BlueprintMapLibrary.Map_Add` _itemtotalscache ItemID _returnvalue_2)
        (return true)))
    (else
      (`BlueprintMapLibrary.Map_Add` (`self.ItemTotalsCache`) ItemID Amount)
      (return true))))