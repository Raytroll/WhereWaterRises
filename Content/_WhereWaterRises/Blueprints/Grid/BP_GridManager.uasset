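; Grid manager Blueprint that registers the level's grids with MapManager at startup.
; On BeginPlay, after a short delay, it finds actors tagged "Grid" and binds each one's AC_GridComponent, printing the result or an invalid-component warning.
; An unconnected debug chain exercises the MapManager API by creating a grid, placing a structure, locating it and testing whether another placement is allowed.
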(event `self.ReceiveBeginPlay`
  (`KismetSystemLibrary.Delay` 0.1)
  (bind _outactors (`GameplayStatics.GetAllActorsWithTag` "Grid"))
  (for _array_element _outactors
    (bind _returnvalue (`self.GetComponentByClass` _array_element "/Game/_WhereWaterRises/Components/AC_GridComponent.AC_GridComponent_C"))
    (`/Engine/EditorBlueprintResources/StandardMacros.IsValid` _returnvalue
      (:`Is Valid`
        (bind _outputpin (`/Game/_WhereWaterRises/Components/AC_MapManager.BindGrid` (`self.MapManager`) _returnvalue))
        (`KismetSystemLibrary.PrintString` (`KismetStringLibrary.Concat_StrStr` "Grid binded: " _outputpin)))
      (:`Is Not Valid`
        (`KismetSystemLibrary.PrintString` "Component not valid")))))

(fn `UserConstructionScript`)