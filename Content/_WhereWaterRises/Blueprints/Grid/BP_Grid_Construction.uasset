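; Grid actor that visualizes a block lattice and lays the starting dirt layer for a map grid.
; The construction script builds a 3D array of small, non-colliding cube meshes at evenly spaced positions as cell markers.
; SetupDirt walks the grid component's placeable blocks and has the passed-in map manager place a BP_Dirt with a new unique hash on each ground-level cell.
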(event `/Game/_WhereWaterRises/Interfaces/GridLogic.SetupDirt`
  (params (MapManager :type "/Game/_WhereWaterRises/Components/AC_MapManager Object Reference") (GridHash :type String))
  (bind _valuepin (`|SetForEach` (`/Game/_WhereWaterRises/Components/AC_GridComponent.PlacableBlocks` (`self.AC_GridComponent`)))
    (:`then`
      (if (== (`.Z_8_45CDE98848859CCA157CC5A7BBE430F3` (break `/Game/_WhereWaterRises/Data/Grid/Struct/F_Vec3I` _valuepin)) 0)
        (bind _hash (`/Game/_WhereWaterRises/Components/AC_MapManager.GenerateUniqueHash` MapManager 16))
        (`/Game/_WhereWaterRises/Components/AC_MapManager.PlaceBuildingFromLocalPosition` MapManager _hash GridHash _valuepin "NewEnumerator0" "/Game/_WhereWaterRises/Blueprints/Building/BP_Dirt.BP_Dirt_C")))))

(fn `UserConstructionScript`
  (for _index (range 9)
    (for _index_2 (range 9)
      (for _index_3 (range 3)
        (bind _returnvalue (`AddComponent|NODE_AddStaticMeshComponent-0` :`RelativeTransform` (`KismetMathLibrary.MakeTransform` (`KismetMathLibrary.MakeVector` (`KismetMathLibrary.Conv_IntToDouble` (* _index 100)) (`KismetMathLibrary.Conv_IntToDouble` (* _index_2 100)) (`KismetMathLibrary.Conv_IntToDouble` (* _index_3 100))) (struct) (0.25 0.25 0.25))))
        (`StaticMeshComponent.SetStaticMesh` _returnvalue "/Engine/BasicShapes/Cube.Cube")
        (`PrimitiveComponent.SetCollisionEnabled` _returnvalue "NoCollision")))))