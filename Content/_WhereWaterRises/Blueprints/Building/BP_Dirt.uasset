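; BP_Dirt is a grid-based dirt building block that tracks an irrigation level and cannot store items or cook.
; On each neighbor update the level decays by one, then refills to a fixed maximum if a watered BP_Goutiere gutter sits directly above.
; Irrigated dirt then spreads a one-lower level to drier dirt neighbors in CheckKernel, forming a falloff gradient.
; A TextRender displays the propagated value.
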(event `self.ReceiveBeginPlay`)

(fn `CanStoreItems`
  (returns (Value :type Boolean))
  (return false))

(fn `Cook`
  (params (Ingredient :type Name))
  (returns (Result :type Name) (Quantity :type Integer))
  (return "None" 0))

(fn `OnUpdate`
  (params (Neighbors :type "Map of /Game/_WhereWaterRises/Data/Grid/Struct/F_Vec3I Structure to Actor Class Reference") (NeighborsActors :type "Map of /Game/_WhereWaterRises/Data/Grid/Struct/F_Vec3I Structure to Actor Object Reference") (NeighborsHashs :type "Map of /Game/_WhereWaterRises/Data/Grid/Struct/F_Vec3I Structure to String") (`Current Cell Hash` :type String) (`Current Cell Hash Orientation` :type "/Game/_WhereWaterRises/Data/Building/Enumerations/E_BuildingOrientation Enum" :default "NewEnumerator0"))
  (returns (BuildingsToAdd :type "Map of /Game/_WhereWaterRises/Data/Grid/Struct/F_Vec3I Structure to Actor Class Reference") (BuildingsToRemove :type "Set of /Game/_WhereWaterRises/Data/Grid/Struct/F_Vec3I Structure"))
  (locals (CheckKernel :type "Set of /Game/_WhereWaterRises/Data/Grid/Struct/F_Vec3I Structure"))
  (bind _f_vec3i (make `/Game/_WhereWaterRises/Data/Grid/Struct/F_Vec3I` 0 0 1))
  (bind _returnvalue (- (`self.IrrigationLevel`) 1))
  (`|ExecutionSequence`
    (:`then_0`
      (set `self.IrrigationLevel` (`KismetMathLibrary.Max` (- (`self.IrrigationLevel`) 1)))
      (if (== (`BlueprintMapLibrary.Map_Find` Neighbors _f_vec3i) "/Game/_WhereWaterRises/Blueprints/Building/BP_Goutiere.BP_Goutiere_C")
        (bind _asbp_goutiere (cast `/Game/_WhereWaterRises/Blueprints/Building/BP_Goutiere` (`BlueprintMapLibrary.Map_Find` NeighborsActors _f_vec3i)))
        (if (`/Game/_WhereWaterRises/Blueprints/Building/BP_Goutiere.IsWatered` _asbp_goutiere)
          (set `self.IrrigationLevel` 4))))
    (:`then_1`
      (if (> (`self.IrrigationLevel`) 0)
        (bind _valuepin (`|SetForEach` (`local.CheckKernel`))
          (:`then`
            (bind _asbp_dirt (cast `/Game/_WhereWaterRises/Blueprints/Building/BP_Dirt` (`BlueprintMapLibrary.Map_Find` NeighborsActors _valuepin)))
            (if (< (`/Game/_WhereWaterRises/Blueprints/Building/BP_Dirt.IrrigationLevel` _asbp_dirt) _returnvalue)
              (bind _output_get (set `/Game/_WhereWaterRises/Blueprints/Building/BP_Dirt.IrrigationLevel` (`KismetMathLibrary.Max` _returnvalue) _asbp_dirt))
              (`TextRenderComponent.K2_SetText` (`self.TextRender`) (`KismetTextLibrary.Conv_IntToText` _output_get))))
          (:`CompletedPin`
            (return)))))))

(fn `UserConstructionScript`)