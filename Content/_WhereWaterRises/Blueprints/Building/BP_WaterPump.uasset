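; BP_WaterPump is a building that spreads water into empty neighboring cells when it sits on water.
; OnUpdate checks the neighbor map for BP_Water directly below, then drops the cells below and above from the map.
; Each remaining neighbor with no building class is returned as a BP_Water entry to add.
; The pump cannot store items.
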(fn `CanStoreItems`
  (returns (Value :type Boolean))
  (return false))

(fn `OnUpdate`
  (params (Neighbors :type "Map of /Game/_WhereWaterRises/Data/Grid/Struct/F_Vec3I Structure to Actor Class Reference") (NeighborsActors :type "Map of /Game/_WhereWaterRises/Data/Grid/Struct/F_Vec3I Structure to Actor Object Reference"))
  (returns (BuildingsToAdd :type "Map of /Game/_WhereWaterRises/Data/Grid/Struct/F_Vec3I Structure to Actor Class Reference") (BuildingsToRemove :type "Set of /Game/_WhereWaterRises/Data/Grid/Struct/F_Vec3I Structure"))
  (locals (BlocksToAdd :type "Map of /Game/_WhereWaterRises/Data/Grid/Struct/F_Vec3I Structure to Actor Class Reference"))
  (bind (_value _returnvalue) (`BlueprintMapLibrary.Map_Find` Neighbors (make `/Game/_WhereWaterRises/Data/Grid/Struct/F_Vec3I` 0 0 -1)))
  (if _returnvalue
    (if (== _value "/Game/_WhereWaterRises/Blueprints/Building/BP_Water.BP_Water_C")
      (`BlueprintMapLibrary.Map_Remove` Neighbors (make `/Game/_WhereWaterRises/Data/Grid/Struct/F_Vec3I` 0 0 -1))
      (`BlueprintMapLibrary.Map_Remove` Neighbors (make `/Game/_WhereWaterRises/Data/Grid/Struct/F_Vec3I` 0 0 1))
      (`BlueprintMapLibrary.Map_Clear` (`local.BlocksToAdd`))
      (bind (_keypin _valuepin) (`|MapForEach` Neighbors)
        (:`then`
          (if (== _valuepin null)
            (`BlueprintMapLibrary.Map_Add` (`local.BlocksToAdd`) _keypin "/Game/_WhereWaterRises/Blueprints/Building/BP_Water.BP_Water_C")))
        (:`CompletedPin`
          (return (`local.BlocksToAdd`))))
      (else
        (return)))))

(fn `UserConstructionScript`)