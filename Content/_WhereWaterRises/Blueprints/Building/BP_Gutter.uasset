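; Gutter building actor that registers itself with the map manager when play begins.
; BeginPlay requests a unique hash from MapManager, packs it into a Building struct and initializes its BuildingComponent with it.
; It then places the building on the hardcoded "Grid_1" grid at the struct's position and prints the placement result for debugging.
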(event `self.ReceiveBeginPlay`
  (bind _hash (`/Game/Structures/MapManager.GenerateUniqueHash` (`self.MapManager`) (`self.Size`)))
  (bind _output_get (set `self.Building` (make `/Game/Structures/Building` _hash)))
  (`/Game/Structures/BuildingComponent.InitBuilding` (`self.BuildingComponent`) _output_get)
  (bind _success (`/Game/Structures/MapManager.PlaceBuilding` (`self.MapManager`) _hash "Grid_1" (`.Pos_13_6C6954234700610B5B44CEAF5FC5EAA0` (break `/Game/Structures/Building` (`self.Building`)))))
  (`KismetSystemLibrary.PrintString` (`KismetStringLibrary.Conv_BoolToString` _success)))

(fn `UserConstructionScript`)