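; Building is a Blueprint, apparently a base for placed buildings, that stores an orientation and looks up machine recipes.
; HandleCellUpdate takes neighbour cells but is empty here, likely a hook for child classes to override.
; GetRecipe scans every row of DT_Recipe for a matching machine class.
; It returns each match as a RecipeInMachine struct holding the row name as result, produced quantity and ingredients.
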(fn `GetRecipe`
  (params (MachineClass :type "Actor Class Reference"))
  (returns (`F Recipe in Machine` :type "Array of /Game/_WhereWaterRises/Data/Recipe/F_RecipeInMachine Structure"))
  (locals (`Recipe in Machine` :type "Array of /Game/_WhereWaterRises/Data/Recipe/F_RecipeInMachine Structure"))
  (bind _outrownames (`DataTableFunctionLibrary.GetDataTableRowNames` "/Game/_WhereWaterRises/Data/Recipe/DT_Recipe.DT_Recipe"))
  (for _array_element _outrownames
    (bind _returnvalue (`|GetDataTableRow` "/Game/_WhereWaterRises/Data/Recipe/DT_Recipe.DT_Recipe" _array_element)
      (:`then`
        (if (== (`.Machine_14_AAED36F5456E2FA2C2B9AF81D8AC999B` (break `/Game/_WhereWaterRises/Data/Recipe/F_Recipe` _returnvalue)) MachineClass)
          (`KismetArrayLibrary.Array_Add` (`local.Recipe in Machine`) (make `/Game/_WhereWaterRises/Data/Recipe/F_RecipeInMachine` _array_element (`.QuantityProduct_9_ACD787E24DA363210AB26380C65C63F9` (break `/Game/_WhereWaterRises/Data/Recipe/F_Recipe` _returnvalue)) (break `/Game/_WhereWaterRises/Data/Recipe/F_Recipe` _returnvalue)))))))
  (return (`local.Recipe in Machine`)))

(fn `HandleCellUpdate`
  (params (NeigbourgCells :type "Map of /Game/_WhereWaterRises/Data/Grid/Struct/F_Vec3I Structure to /Game/_WhereWaterRises/Blueprints/Building Object Reference"))
  (locals (CheckList :type Boolean)))

(fn `SetOrientation`
  (params (Orientation :type "/Game/_WhereWaterRises/Data/Building/Enumerations/E_BuildingOrientation Enum" :default "NewEnumerator0"))
  (set `self.Orientation` Orientation))