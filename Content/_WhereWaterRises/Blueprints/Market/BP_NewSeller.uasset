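; BP_NewSeller spawns market sellers stocked with randomly picked items from a price map.
; CreateNewSeller, while free positions remain, adds a few random picks from PriceItemToSell to a price map and a unique item list.
; It spawns a BP_Seller at the first position, passes it both collections, builds its inventory and removes that position.
; Neither collection is cleared here, so picks accumulate across calls.
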(event `CreateNewSeller`
  (bind (_key _value) (`BlueprintMapLibrary.Map_GetKeyValueByIndex` (`self.Price Item_ToSell`) (`KismetMathLibrary.RandomIntegerInRange` 0 (`BlueprintMapLibrary.Map_Length` (`self.Price Item_ToSell`)))))
  (if (> (`KismetArrayLibrary.Array_Length` (`self.Position Seller`)) 0)
    (for _ (range (+ (`KismetMathLibrary.RandomIntegerInRange` 1 3) 1))
      (`BlueprintMapLibrary.Map_Add` (`self.Price Item`) _key _value)
      (`KismetArrayLibrary.Array_AddUnique` (`self.List Item to Sell`) _key))
    (bind _returnvalue (`|SpawnActorFromClass` "/Game/_WhereWaterRises/Blueprints/Market/BP_Seller.BP_Seller_C" (`KismetMathLibrary.MakeTransform` (`|GetArrayItem` (`self.Position Seller`))) "AdjustIfPossibleButAlwaysSpawn" "MultiplyWithRoot" null null))
    (`/Engine/EditorBlueprintResources/StandardMacros.IsValid` _returnvalue
      (:`Is Valid`
        (`/Game/_WhereWaterRises/Blueprints/Market/BP_Seller.SetInventoryWidget` _returnvalue (`self.Price Item`) (`self.List Item to Sell`))
        (`/Game/_WhereWaterRises/Blueprints/Market/BP_Seller.CreateInventory` _returnvalue)
        (`KismetArrayLibrary.Array_Remove` (`self.Position Seller`))))))

(fn `UserConstructionScript`)