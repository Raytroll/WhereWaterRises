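; Market seller actor that opens a trade menu on player interaction and shows a prompt widget while something overlaps its interaction area.
; CreateInventory builds the trade widget and fills it and the seller's inventory component from DT_Items rows, with Limited false for every item type.
; OnPlayerHit and CloseWidgetMarket share one toggle that adds or removes the menu and switches input mode, mouse capture and cursor.
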(event `CreateInventory`
  ;[0.15 0.02181 0.02374 0.5] Setup Seller Inventory
  (bind _returnvalue (`|CreateWidget` "/Game/_WhereWaterRises/Blueprints/Market/WBP_TradeMenu.WBP_TradeMenu_C" null (`self.Price Item`)))
  (bind _output_get (set `self.ParentWidget` _returnvalue))
  (`Widget.SetKeyboardFocus` (`/Game/_WhereWaterRises/Blueprints/Market/WBP_TradeMenu.Close` _output_get))
  (for _array_element (`self.ListItemToSell`)
    (bind _returnvalue_2 (`|GetDataTableRow` "/Game/_WhereWaterRises/Blueprints/PlayerInventory/Data/DT_Items.DT_Items" _array_element)
      (:`then`
        (if (`|EnumEquality` (`.Type_22_65850FF046D3117DC61602B0F5578CBD` (break `/Game/_WhereWaterRises/Blueprints/PlayerInventory/Data/F_ItemData` _returnvalue_2)) "NewEnumerator1")
          (set `self.Limited?` false)
          (else
            (set `self.Limited?` false)))
        (bind _quantityaccepted (`/Game/_WhereWaterRises/Blueprints/PlayerInventory/AC_InventoryComponent.CanAddItem` (`self.AC_InventoryComponent`) _array_element 1))
        (`/Game/_WhereWaterRises/Blueprints/PlayerInventory/AC_InventoryComponent.AddItem` (`self.AC_InventoryComponent`) _array_element _quantityaccepted)
        (`/Game/_WhereWaterRises/Blueprints/Market/WBP_TradeMenu.SetInventory` (`self.ParentWidget`) (`self.Limited?`) _array_element)))))

(event `CloseWidgetMarket`
  (bind _returnvalue (`GameplayStatics.GetPlayerController` 0))
  (bind _parentwidget (`self.ParentWidget`))
  ;[0.15 0.0561 0.1368 0.5] Open Menu Trade / lose Menu Trade
  (if (`self.MenuOpen?`) :!label _label
    (`GameplayStatics.SetViewportMouseCaptureMode` "CapturePermanently_IncludingInitialMouseDown")
    (`WidgetBlueprintLibrary.SetInputMode_GameOnly` _returnvalue true)
    (set `PlayerController.bShowMouseCursor` false _returnvalue)
    (`Widget.RemoveFromParent` (`self.ParentWidget`))
    (set `self.MenuOpen?` false)
    (else
      (`/Game/_WhereWaterRises/Blueprints/Market/WBP_TradeMenu.SetSeller` _parentwidget self)
      (`UserWidget.AddToViewport` _parentwidget 0)
      (set `self.MenuOpen?` true)
      (`GameplayStatics.SetViewportMouseCaptureMode` "NoCapture")
      (`WidgetBlueprintLibrary.SetInputMode_UIOnlyEx` _returnvalue (`/Game/_WhereWaterRises/Blueprints/Market/WBP_TradeMenu.Close` _parentwidget) "DoNotLock" true)
      (set `PlayerController.bShowMouseCursor` true _returnvalue))))

(event `OnPlayerHit`
  ;[0.15 0.0561 0.1368 0.5] Open Menu Trade / lose Menu Trade
  (goto _label))

(event `self.Interactable area.OnComponentBeginOverlap`
  (params (OverlappedComponent :type "PrimitiveComponent Object Reference") (OtherActor :type "Actor Object Reference") (OtherComp :type "PrimitiveComponent Object Reference") (OtherBodyIndex :type Integer) (bFromSweep :type Boolean) (SweepResult :type "HitResult Structure (by ref)"))
  (`SceneComponent.SetVisibility` (`self.Widget_Interaction`) true false))

(event `self.Interactable area.OnComponentEndOverlap`
  (params (OverlappedComponent :type "PrimitiveComponent Object Reference") (OtherActor :type "Actor Object Reference") (OtherComp :type "PrimitiveComponent Object Reference") (OtherBodyIndex :type Integer))
  (`SceneComponent.SetVisibility` (`self.Widget_Interaction`) false false))

(fn `SetInventoryInWidget`
  (returns (`Price Item1` :type "Map of Name to /Game/_WhereWaterRises/Blueprints/Market/S_Price Structure"))
  (return (`self.Price Item`)))

(fn `SetInventoryWidget`
  (params (`Price Item` :type "Map of Name to /Game/_WhereWaterRises/Blueprints/Market/S_Price Structure") (ListItemToSell :type "Array of Name"))
  (set `self.Price Item` `Price Item`)
  (set `self.ListItemToSell` ListItemToSell))

(fn `UserConstructionScript`)