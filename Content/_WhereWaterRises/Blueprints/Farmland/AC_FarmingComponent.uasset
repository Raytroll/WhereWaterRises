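; Farming component that plants crops on the grid and tracks them by placement hash in ActiveCrops.
; PlantSeed validates the cell through the map manager, places a BP_Farmland building and stores its crop state.
; Tick loops over crops for a water-edge boost, but the growth write-back is unwired.
; Chebyshev-distance water boost is drafted but not called here; CalculateInitialBoost is a stub, and ItemCanBePlanted maps items to crops.
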(event `self.ReceiveBeginPlay`
  (bind _returnvalue (`GameplayStatics.GetActorOfClass` "/Game/_WhereWaterRises/Blueprints/Grid/BP_GridManager.BP_GridManager_C"))
  (set `self.Ref_MapManager` _returnvalue)
  (bind _returnvalue_2 (`GameplayStatics.GetActorOfClass` "/Game/_WhereWaterRises/Blueprints/Farmland/BP_Farmland.BP_Farmland_C"))
  (set `self.Ref_GridComponent` (`Actor.GetComponentByClass` _returnvalue_2 "/Game/_WhereWaterRises/Components/AC_GridComponent.AC_GridComponent_C")))

(event `self.ReceiveTick`
  (params (DeltaSeconds :type "Float (single-precision)"))
  (`self.UpdateGrowthTime` DeltaSeconds))

(fn `CalculateInitialBoost`
  (params (GridPosition :type "/Game/_WhereWaterRises/Data/Grid/Struct/F_Vec3I Structure"))
  (returns (BoostMultiplier :type "Float (double-precision)"))
  (locals (Local_TempMultiplier :type "Float (double-precision)" :default 1.0))
  (for _ (range (`KismetMathLibrary.Clamp` (`.X_6_C46BC9A74AEFAF411D89D0A533D7FC68` (break `/Game/_WhereWaterRises/Data/Grid/Struct/F_Vec3I` GridPosition)) -1 1) 2)
    _))

(fn `CalculateWaterProximityBoost`
  (params (CropKey :type String))
  (returns (BoostMultiplier :type "Float (double-precision)"))
  (locals (Local_BestDistance :type Integer))
  (bind (_position _found) (`/Game/_WhereWaterRises/Components/AC_GridComponent.FindBlockPositionByHash` (`self.Ref_GridComponent`) CropKey))
  (if _found
    (set `local.Local_BestDistance` (+ (`self.WaterBoostRange`) 1))
    (bind _keypin (`|MapForEach` (`/Game/_WhereWaterRises/Components/AC_GridComponent.BlocksWaterIsEdge` (`self.Ref_GridComponent`)))
      (:`then`
        (bind (_position_2 _found_2) (`/Game/_WhereWaterRises/Components/AC_GridComponent.FindBlockPositionByHash` (`self.Ref_GridComponent`) _keypin))
        (if _found_2
          (bind (_x _y) (break `/Game/_WhereWaterRises/Data/Grid/Struct/F_Vec3I` _position))
          (bind (_x_2 _y_2) (break `/Game/_WhereWaterRises/Data/Grid/Struct/F_Vec3I` _position_2))
          (bind _returnvalue (`KismetMathLibrary.Max` (`KismetMathLibrary.Abs_Int` (- _x _x_2)) (`KismetMathLibrary.Abs_Int` (- _y _y_2))))
          (if (< (`local.Local_BestDistance`) _returnvalue)
            (bind _output_get (set `local.Local_BestDistance` _returnvalue))
            (if (> _output_get (`self.WaterBoostRange`))
              (return 1.0)
              (else
                (return (`KismetMathLibrary.Lerp` (`self.MaxBoostMultiplier`) 1.0 (`KismetMathLibrary.Conv_IntToDouble` (/ (`local.Local_BestDistance`) (`self.WaterBoostRange`)))))))))))))

(fn `ItemCanBePlanted`
  (params (ItemID :type Name))
  (returns (CropData :type "/Game/_WhereWaterRises/Blueprints/Farmland/Data/DA_BaseCropData Object Reference"))
  (bind (_value _returnvalue) (`BlueprintMapLibrary.Map_Find` (`self.ItemToCropMap`) ItemID))
  (if _returnvalue
    (return _value)
    (else
      (return null))))

(fn `PlantSeed`
  (params (WorldLocation :type "Vector Structure") (CropDataAsset :type "/Game/_WhereWaterRises/Blueprints/Farmland/Data/DA_BaseCropData Object Reference"))
  (returns (bIsEmptyCase :type Boolean))
  (bind _mapmanager (`/Game/_WhereWaterRises/Blueprints/Grid/BP_GridManager.MapManager` (`self.Ref_MapManager`)))
  (`/Engine/EditorBlueprintResources/StandardMacros.IsValid` CropDataAsset
    (:`Is Valid`
      (bind _outputpin (`/Game/_WhereWaterRises/Components/AC_MapManager.BindGrid` _mapmanager (`self.Ref_GridComponent`)))
      (bind (_postitionongrid _worldtransformongrid _success) (`/Game/_WhereWaterRises/Components/AC_MapManager.ProjectPointOntoGridSpace` _mapmanager WorldLocation _outputpin))
      (if _success
        (bind _success_2 (`/Game/_WhereWaterRises/Components/AC_MapManager.CanPlaceBuildingOnGridAtPosition` _mapmanager _outputpin _postitionongrid))
        (if _success_2
          (bind (_hash _success_3) (`/Game/_WhereWaterRises/Components/AC_MapManager.PlaceBuildingFromWorldPosition` _mapmanager _outputpin WorldLocation "NewEnumerator0" "/Game/_WhereWaterRises/Blueprints/Farmland/BP_Farmland.BP_Farmland_C"))
          (if _success_3
            (if (not (`.ReturnValue` (`BlueprintMapLibrary.Map_Find` (`self.Active Crops`) _hash)))
              (`BlueprintMapLibrary.Map_Add` (`self.Active Crops`) _hash (make `/Game/_WhereWaterRises/Blueprints/Farmland/Data/F_CropState` CropDataAsset 0.0 0.0 1.0))
              (return true))))))))

(fn `UpdateGrowthTime`
  (params (DeltaTime :type "Float (double-precision)"))
  (locals (Local_DeltaTime :type "Float (double-precision)") (Local_CurrentBoost :type "Float (double-precision)"))
  (set `local.Local_DeltaTime` DeltaTime)
  (bind (_keypin _valuepin) (`|MapForEach` (`self.Active Crops`))
    (:`then`
      (if (`BlueprintMapLibrary.Map_Find` (`/Game/_WhereWaterRises/Components/AC_GridComponent.BlocksWaterIsEdge` (`self.Ref_GridComponent`)) _keypin)
        (set `local.Local_CurrentBoost` (* (`.BoostMultiplier_17_6279F31247FDDCED4CBA24B8A5C67ED5` (break `/Game/_WhereWaterRises/Blueprints/Farmland/Data/F_CropState` _valuepin)) 1.5))))))