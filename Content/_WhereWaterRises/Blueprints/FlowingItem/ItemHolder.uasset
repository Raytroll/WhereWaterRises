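; ItemHolder is an actor representing an item that flows between cells, showing its icon on a plane.
; SetItemType looks up DT_Items and applies the row's icon through a dynamic material instance, defaulting to sand on construction.
; Tick counts down a flow cooldown, set to at least one second, and eases the actor toward TargetPosition with a per-frame lerp.
; CanFlowToNext requires an expired cooldown and refuses the previous cell's hash, preventing backflow.
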(event `self.ReceiveTick`
  (params (DeltaSeconds :type "Float (single-precision)"))
  (set `self.FlowCooldown` (`KismetMathLibrary.FMax` (- (`self.FlowCooldown`) DeltaSeconds)))
  (`SceneComponent.K2_SetWorldLocation` (`self.DefaultSceneRoot`) (`KismetMathLibrary.VLerp` (`SceneComponent.K2_GetComponentLocation` (`self.DefaultSceneRoot`)) (`self.TargetPosition`) 0.1) false false))

(fn `CanFlowToNext`
  (params (`Requesting Cell Hash` :type String))
  (returns (CanFlow :type Boolean))
  (return (and (`KismetStringLibrary.NotEqual_StrStr` `Requesting Cell Hash` (`self.Previous Cell Hash`)) (<= (`self.FlowCooldown`) 0.0))))

(fn `IsReady`
  (returns (IsReady :type Boolean))
  (return (<= (`self.FlowCooldown`) 0.0)))

(fn `SetCooldown`
  (params (Value :type "Float (double-precision)"))
  (set `self.FlowCooldown` (`KismetMathLibrary.FMax` Value 1.0)))

(fn `SetItemQuantity`
  (params (Quantity :type Integer))
  (set `self.Quantity` Quantity))

(fn `SetItemType`
  (params (Name :type Name))
  (bind _output_get (set `self.ItemType` Name))
  (bind _returnvalue (`|GetDataTableRow` "/Game/_WhereWaterRises/Blueprints/PlayerInventory/Data/DT_Items.DT_Items" _output_get)
    (:`then`
      (bind _returnvalue_2 (`PrimitiveComponent.CreateDynamicMaterialInstance` (`self.Plane`) 0 "/Game/_WhereWaterRises/Blueprints/FlowingItem/Item_MAT.Item_MAT" "None"))
      (`MaterialInstanceDynamic.SetTextureParameterValue` _returnvalue_2 "IconTexture" (`.Icon_24_C2AA87E34672B51096A2E3A1F61D6ED4` (break `/Game/_WhereWaterRises/Blueprints/PlayerInventory/Data/F_ItemData` _returnvalue)))
      (`PrimitiveComponent.SetMaterial` (`self.Plane`) 0 _returnvalue_2))))

(fn `SetPreviousCell`
  (params (Hash :type String))
  (set `self.Previous Cell Hash` Hash))

(fn `UserConstructionScript`
  (`self.SetItemType` "ID_sand")
  (`self.SetCooldown` 0.0))