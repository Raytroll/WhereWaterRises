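; AC_Craft_Test is a crafting test that checks a recipe against the inventory of the BP_Iddin-Nabu player pawn.
; It caches that pawn's ACInventoryComponent on BeginPlay.
; CanCraft? loops over a recipe map of item IDs to quantities, calls CanRemoveItem without using its result, then removes the item.
; It returns inside the loop, so only the first ingredient is consumed and decides IsCraftable and QuantityRemoved.
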(event `self.ReceiveBeginPlay`
  (bind _asbp_iddin__nabu (cast `/Game/_WhereWaterRises/Characters/Blueprints/BP_Iddin-Nabu` (`GameplayStatics.GetPlayerPawn` 0)))
  (set `self.AC Inventory Component` (`/Game/_WhereWaterRises/Characters/Blueprints/BP_Iddin-Nabu.AC_InventoryComponent` _asbp_iddin__nabu)))

(fn `CanCraft?`
  (params (Recipe :type "Map of Name to Integer"))
  (returns (QuantityRemoved :type Integer) (`IsCraftable?` :type Boolean))
  (bind (_keypin _valuepin) (`|MapForEach` Recipe)
    (:`then`
      (`/Game/_WhereWaterRises/Blueprints/PlayerInventory/AC_InventoryComponent.CanRemoveItem` (`self.AC Inventory Component`) _keypin _valuepin)
      (bind (_quantityremoved _quantityremaining _issuccess) (`/Game/_WhereWaterRises/Blueprints/PlayerInventory/AC_InventoryComponent.RemoveItem` (`self.AC Inventory Component`) _keypin _valuepin))
      (return _quantityremoved _issuccess))))