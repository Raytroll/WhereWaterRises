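; AC_ActionSystem is an actor component that tracks a pool of action points for its owner.
; UsePoint and RefundPoint lower or raise the current points by one, clamped between zero and the maximum.
; HasEnoughPts checks whether the current points cover a given amount, and ResetPoint refills the pool to the maximum.
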(fn `HasEnoughPts?`
  (params (Amount :type "Float (double-precision)"))
  (returns (`HasPoint?` :type Boolean))
  ; Check if has enough action point?
  (if (>= (`self.CurrentPts`) Amount)
    (return true)
    (else
      (return false))))

(fn `RefundPoint`
  ; Using point
  (set `self.CurrentPts` (`KismetMathLibrary.FClamp` (+ (`self.CurrentPts`) 1.0) 0.0 (`self.MaxPts`))))

(fn `ResetPoint`
  (set `self.CurrentPts` (`self.MaxPts`)))

(fn `UsePoint`
  ; Using point
  (set `self.CurrentPts` (`KismetMathLibrary.FClamp` (- (`self.CurrentPts`) 1.0) 0.0 (`self.MaxPts`))))